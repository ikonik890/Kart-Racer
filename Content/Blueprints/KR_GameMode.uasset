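; KR_GameMode is a game mode that gives joining players varied pawns and separate spawn points.
; On each player restart event it sets DefaultPawnClass from the PlayerPawns array, cycling by an incrementing PlayerCount with modulo.
; The ChoosePlayerStart override returns the first PlayerStart not tagged "Used" and tags it, so starts are never released for reuse.
; An unconnected branch that assigns per-player meshes to ThunderstruckPawn never runs.
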(event `self.K2_OnRestartPlayer`
  (params (NewPlayer :type "Controller Object Reference"))
  (bind _playerpawns (`self.PlayerPawns`))
  (set `self.DefaultPawnClass` (`|GetArrayItem` _playerpawns (mod (`self.PlayerCount`) (`KismetArrayLibrary.Array_Length` _playerpawns))))
  (`/Engine/EditorBlueprintResources/StandardMacros.IncrementInt` (`self.PlayerCount`)))

(fn `ChoosePlayerStart`
  (params (Player :type "Controller Object Reference"))
  (returns (ReturnValue :type "Actor Object Reference"))
  (bind _outactors (`GameplayStatics.GetAllActorsOfClass` "/Script/Engine.PlayerStart"))
  (for _array_element _outactors
    (bind _asplayer_start (cast `PlayerStart` _array_element))
    (if (!= (`PlayerStart.PlayerStartTag` _asplayer_start) "Used")
      (set `PlayerStart.PlayerStartTag` "Used" _asplayer_start)
      (return _asplayer_start))))

(fn `UserConstructionScript`)